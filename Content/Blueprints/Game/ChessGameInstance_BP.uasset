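; Game instance for a chess game that handles hosting, joining and browsing two-player multiplayer sessions.
; Hosting creates a session with optional LAN and opens the chess map as a listen server, while joining connects to a supplied search result.
; Searching requests a state change, then shows a reusable server list widget with UI-only input.
; Main menu, network and travel error events, ChangeState and ShowError are unimplemented stubs.
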(event `OnShowMainMenu`)

(event `OnHostGame`
  ;[1 1 1] Host game
  (`CreateSessionCallbackProxy.CreateSession` (`GameplayStatics.GetPlayerController` 0) 2 (`self.UseLAN`)
    (:`OnSuccess`
      (`GameplayStatics.OpenLevel` "ChessGameMap" true "listen"))
    (:`OnFailure`
      (`self.ShowError` "Failed to create session"))))

(event `OnJoinGame`
  (params (Session :type "BlueprintSessionResult Structure"))
  ;[1 1 1] Join game
  (`JoinSessionCallbackProxy.JoinSession` (`GameplayStatics.GetPlayerController` 0) Session
    (:`OnFailure`
      (`self.ShowError` "Failed to join session"))))

(event `self.HandleNetworkError`
  (params (FailureType :type "ENetworkFailure Enum" :default "NetDriverAlreadyExists") (bIsServer :type Boolean)))

(event `self.HandleTravelError`
  (params (FailureType :type "ETravelFailure Enum" :default "NoLevel")))

(event `OnSearchGames`
  (bind _returnvalue (`GameplayStatics.GetPlayerController` 0))
  ;[1 1 1] Searching games
  (`self.ChangeState` "SEARCH_SERVER"
    (:`O`
      (`/Engine/EditorBlueprintResources/StandardMacros.IsValid` (`self.ServerList`)
        (:`Is Valid`
          _)
        (:`Is Not Valid`
          (bind _returnvalue_2 (`|CreateWidget` "/Game/HUD/ServerList.ServerList_C" _returnvalue))
          (bind _output_get (set `self.ServerList` _returnvalue_2))))
      (`UserWidget.AddToViewport` _output_get 1)
      (`WidgetBlueprintLibrary.SetInputMode_UIOnlyEx` _returnvalue _output_get))))