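; MoveHintPlane_BP is a board actor that, judging by its name, serves as a plane marking a move hint.
; Its construction script pins the actor's Z location to just above zero, keeping X, Y, rotation and scale.
; BeginPlay and Tick are empty; leftover unconnected nodes would create a dynamic material, set its Emissive parameter and stop ticking after a timer, but never run.
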(event `self.ReceiveBeginPlay`)

(event `self.ReceiveTick`
  (params (DeltaSeconds :type "Float (single-precision)")))

(fn `UserConstructionScript`
  (bind _returnvalue (`self.GetTransform`))
  (`self.K2_SetActorTransform` (`KismetMathLibrary.MakeTransform` (`KismetMathLibrary.MakeVector` (.x (.location _returnvalue)) (.y (.location _returnvalue)) 0.1) (.rotation _returnvalue) (.scale _returnvalue))))